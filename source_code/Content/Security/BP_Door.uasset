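; BP_Door is a sliding security door that shuts on its CloseDoor event and reopens automatically after a five-second delay.
; The Left flag picks the slide direction and distance, with separate close and reopen timelines for each side lerping the door's relative Y.
; IsClosedLeft or IsClosedRight tracks the state.
; The flags, delay and reopen call all hang off timeline Update pins rather than Finished.
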(event `CloseDoor`
  (if (`self.left`)
    (bind (_direction _doorfloat) (`Timeline|CloseDoorTimeline` :!via `PlayFromStart`)
      (:`Update`
        (`SceneComponent.K2_SetRelativeLocation` (`self.Door`) (`KismetMathLibrary.MakeVector` 0.0 (`KismetMathLibrary.Lerp` 0.0 -250.0 _doorfloat)) false false)
        (set `self.isClosedLeft` true)
        (`KismetSystemLibrary.Delay` 5.0)
        (bind (_direction_2 _doorfloat_2) (`Timeline|OpenDoorTimeline` :!via `PlayFromStart`)
          (:`Update`
            (`SceneComponent.K2_SetRelativeLocation` (`self.Door`) (`KismetMathLibrary.MakeVector` 0.0 (`KismetMathLibrary.Lerp` 0.0 -250.0 _doorfloat_2)) false false)
            (set `self.isClosedLeft` false)))))
    (else
      (bind (_direction_3 _doorfloat_3) (`Timeline|Timeline` :!via `PlayFromStart`)
        (:`Update`
          (`SceneComponent.K2_SetRelativeLocation` (`self.Door`) (`KismetMathLibrary.MakeVector` 0.0 (`KismetMathLibrary.Lerp` 0.0 450.0 _doorfloat_3)) false false)
          (set `self.isClosedRight` true)
          (`KismetSystemLibrary.Delay` 5.0)
          (bind (_direction_4 _doorfloat_4) (`Timeline|Timeline_0` :!via `PlayFromStart`)
            (:`Update`
              (`SceneComponent.K2_SetRelativeLocation` (`self.Door`) (`KismetMathLibrary.MakeVector` 0.0 (`KismetMathLibrary.Lerp` 0.0 450.0 _doorfloat_4)) false false)
              (set `self.isClosedRight` false))))))))

(fn `UserConstructionScript`)