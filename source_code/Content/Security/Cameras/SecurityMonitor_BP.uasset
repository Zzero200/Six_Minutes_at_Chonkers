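; Security monitor that shows the live feed and name of one security camera from its list, starting with the first.
; A dynamic material displays a render target sized from the viewport and that camera's Quality, fed by its scene capture.
; SwapCamera cycles with wraparound, clearing the old camera's target and creating a new one for the next.
; PlayerInput forwards horizontal and vertical input to rotate the current camera.
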(event `self.ReceiveBeginPlay`
  (bind (_returnvalue_x _returnvalue_y) (`KismetMathLibrary.BreakVector2D` (`WidgetLayoutLibrary.GetViewportSize`)))
  (bind _quality (`/Game/Security/Cameras/SecurityCamera_BP.Quality` (`|GetArrayItem` (`self.Cameras`))))
  (`KismetSystemLibrary.Delay` 0.5)
  (`/Engine/EditorBlueprintResources/StandardMacros.IsValid` (`|GetArrayItem` (`self.Cameras`))
    (:`Is Valid`
      (bind _returnvalue (`KismetMaterialLibrary.CreateDynamicMaterialInstance` "/Game/Security/Cameras/SecurityCamera_MAT.SecurityCamera_MAT" "CameraTexture"))
      (bind _output_get (set `self.CameraMaterial` _returnvalue))
      (`PrimitiveComponent.SetMaterial` (`self.Monitor`) 0 _output_get)
      (bind _returnvalue_2 (`KismetRenderingLibrary.CreateRenderTarget2D` (`KismetMathLibrary.FTrunc` (* _returnvalue_x _quality)) (`KismetMathLibrary.FTrunc` (* _returnvalue_y _quality))))
      (bind _output_get_2 (set `self.CameraRender` _returnvalue_2))
      (bind _output_get_3 (set `SceneCaptureComponent2D.TextureTarget` _output_get_2 (`/Game/Security/Cameras/SecurityCamera_BP.SceneCaptureComponent2D` (`|GetArrayItem` (`self.Cameras`)))))
      (`MaterialInstanceDynamic.SetTextureParameterValue` (`self.CameraMaterial`) "CameraTexture" _output_get_3)
      (`MaterialInstanceDynamic.SetScalarParameterValue` (`self.CameraMaterial`) "Brightness" (`self.Brightness`))
      (`TextRenderComponent.K2_SetText` (`self.CameraName`) (`KismetTextLibrary.Conv_StringToText` (`/Game/Security/Cameras/SecurityCamera_BP.Name` (`|GetArrayItem` (`self.Cameras`))))))))

(event `SwapCamera`
  (params (inReverse :type Boolean))
  (bind (_returnvalue_x _returnvalue_y) (`KismetMathLibrary.BreakVector2D` (`WidgetLayoutLibrary.GetViewportSize`)))
  (bind _currentcamera (`self.CurrentCamera`))
  (bind _returnvalue (`KismetArrayLibrary.Array_Length` (`self.Cameras`)))
  (bind _quality (`/Game/Security/Cameras/SecurityCamera_BP.Quality` (`|GetArrayItem` (`self.Cameras`) (`self.CurrentCamera`))))
  (set `SceneCaptureComponent2D.TextureTarget` null (`/Game/Security/Cameras/SecurityCamera_BP.SceneCaptureComponent2D` (`|GetArrayItem` (`self.Cameras`) (`self.CurrentCamera`))))
  (if inReverse
    (`/Engine/EditorBlueprintResources/StandardMacros.DecrementInt` _currentcamera
      (:`  `
        (if (< _currentcamera 0)
          (bind _result (`/Engine/EditorBlueprintResources/StandardMacros.DecrementInt` _returnvalue)
            (:`  `
              (set `self.CurrentCamera` _result))))))
    (else
      (`/Engine/EditorBlueprintResources/StandardMacros.IncrementInt` _currentcamera
        (:`  `
          (if (>= _currentcamera _returnvalue)
            (set `self.CurrentCamera` 0))))))
  (bind _returnvalue_2 (`KismetRenderingLibrary.CreateRenderTarget2D` (`KismetMathLibrary.FTrunc` (* _returnvalue_x _quality)) (`KismetMathLibrary.FTrunc` (* _returnvalue_y _quality))))
  (bind _output_get (set `self.CameraRender` _returnvalue_2))
  (bind _output_get_2 (set `SceneCaptureComponent2D.TextureTarget` _output_get (`/Game/Security/Cameras/SecurityCamera_BP.SceneCaptureComponent2D` (`|GetArrayItem` (`self.Cameras`) (`self.CurrentCamera`)))))
  (`MaterialInstanceDynamic.SetTextureParameterValue` (`self.CameraMaterial`) "CameraTexture" _output_get_2)
  (`TextRenderComponent.K2_SetText` (`self.CameraName`) (`KismetTextLibrary.Conv_StringToText` (`/Game/Security/Cameras/SecurityCamera_BP.Name` (`|GetArrayItem` (`self.Cameras`) (`self.CurrentCamera`))))))

(event `PlayerInput`
  (params (Horizontal :type "Float (double-precision)") (Vertical :type "Float (double-precision)"))
  (`/Game/Security/Cameras/SecurityCamera_BP.RotateCam` (`|GetArrayItem` (`self.Cameras`) (`self.CurrentCamera`)) Horizontal Vertical))

(fn `UserConstructionScript`)