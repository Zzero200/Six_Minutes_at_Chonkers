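; Security camera actor that can be panned and tilted through a scene capture component.
; RotateCam adds horizontal and vertical input, scaled by per-axis sensitivity, to the SceneCaptureComponent2D's relative rotation.
; Pitch and yaw are clamped to configurable limits and roll is held at zero.
; The event graph and construction script are empty, so rotation happens only when RotateCam is called.
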(fn `RotateCam`
  (params (HorizontalShift :type "Float (double-precision)") (VerticalShift :type "Float (double-precision)"))
  (bind (_relativerotation_roll _relativerotation_pitch _relativerotation_yaw) (`KismetMathLibrary.BreakRotator` (`SceneComponent.RelativeRotation` (`self.SceneCaptureComponent2D`))))
  (`SceneComponent.K2_SetRelativeRotation` (`self.SceneCaptureComponent2D`) (`KismetMathLibrary.MakeRotator` 0.0 (`KismetMathLibrary.FClamp` (+ _relativerotation_pitch (* (`local.VerticalShift`) (`self.VerticalSensitivity`))) (`self.MaxDownRotation`) (`self.MaxUpRotation`)) (`KismetMathLibrary.FClamp` (+ _relativerotation_yaw (* (`local.HorizontalShift`) (`self.HorizontalSensitivity`))) (`self.MaxLeftRotation`) (`self.MaxRightRotation`))) false false))

(fn `UserConstructionScript`)